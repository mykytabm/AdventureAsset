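; Interactable door that slides its static mesh between closed and opened positions each time it receives Interact.
; On BeginPlay it derives both positions from the mesh's starting relative location, the initial Closed flag and OpenCloseDelta, which is subtracted in either case.
; A timeline lerps from the mesh's current location toward the target, then flips Closed and the target.
; A Busy flag ignores interaction mid-move.
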(event `self.ReceiveBeginPlay`
  ;[1 1 1] Event Beginplay; Set Door Open/Close locations based on whether door is closed at the start or not
  (`parent.ReceiveBeginPlay`)
  (`self.SetDoorLocationVariables`))

(event `self.Interact`
  (params (InteractingActor :type "Actor Object Reference"))
  ;[1 1 1] Event Interact; if not Busy set Busy to true and call Use Door
  (if (not (`self.Busy?`))
    (set `self.Busy?` true)
    (`self.UseDoor`)))

(event `UseDoor`
  ;[1 1 1] Event Use Door; Lerp static mesh location to target location, switch target location
  (bind (_direction _lerpalpha) (`Timeline|OpenDoorTL` :!via `PlayFromStart`)
    (:`Update`
      (`SceneComponent.K2_SetRelativeLocation` (`self.StaticMesh`) (`KismetMathLibrary.VLerp` (`SceneComponent.RelativeLocation` (`self.StaticMesh`)) (`self.TargetLocation`) _lerpalpha) false false))
    (:`Finished`
      (`self.ToggleDoorClosed`)
      (set `self.Busy?` false))))

(fn `SetDoorLocationVariables`
  (bind _relativelocation (`SceneComponent.RelativeLocation` (`self.StaticMesh`)))
  (if (`self.Closed?`)
    (bind _output_get (set `self.ClosedLocation` _relativelocation))
    (bind _output_get_2 (set `self.OpenedLocation` (- _output_get (`self.Open/CloseDelta`))))
    (set `self.TargetLocation` _output_get_2)
    (else
      (bind _output_get_3 (set `self.OpenedLocation` _relativelocation))
      (bind _output_get_4 (set `self.ClosedLocation` (- _output_get_3 (`self.Open/CloseDelta`))))
      (set `self.TargetLocation` _output_get_4))))

(fn `ToggleDoorClosed`
  (bind _output_get (set `self.Closed?` (not (`self.Closed?`))))
  (set `self.TargetLocation` (select `bool` _output_get :`false` (`self.ClosedLocation`) :`true` (`self.OpenedLocation`))))

(fn `UserConstructionScript`
  (`parent.UserConstructionScript`))