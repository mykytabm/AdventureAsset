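; Puzzle manager that triggers its target actors when all of its swap tiles are active at the same time.
; On BeginPlay it binds to each tile's OnTileToggled event and keeps a running count of active tiles from those toggles.
; Once the all-active check passes, it unbinds from every tile so the puzzle stops responding, then calls InvokeTargetActors.
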(event `self.ReceiveBeginPlay`
  ;[1 1 1] Event Beginplay; bind swap tiles on Toggled event
  (for _array_element (`self.SwapTiles`)
    (add `/Game/AdventurePack/Blueprints/Interactables/SwapColorTile.OnTileToggled` _array_element (delegate `OnTileToggled_Event_0`))))

(event `OnTileToggled_Event_0`
  (params (`Active?` :type Boolean))
  ;[1 1 1] OnTileToggledEvent
  (`self.CountActiveTiles` `Active?`)
  (if (`self.AllTilesAreActive`)
    (for _array_element (`self.SwapTiles`)
      (remove `/Game/AdventurePack/Blueprints/Interactables/SwapColorTile.OnTileToggled` _array_element (delegate `OnTileToggled_Event_0`)))
    (`self.InvokeTargetActors` self)))

(fn `CountActiveTiles`
  (params (`Active?` :type Boolean))
  (if `Active?`
    (`/Engine/EditorBlueprintResources/StandardMacros.IncrementInt` (`self.ActiveTiles`))
    (else
      (`/Engine/EditorBlueprintResources/StandardMacros.DecrementInt` (`self.ActiveTiles`)))))

(fn `UserConstructionScript`
  (`parent.UserConstructionScript`))