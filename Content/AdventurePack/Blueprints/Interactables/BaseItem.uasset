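; BaseItem is an interactable item actor that can be picked up into an inventory.
; On BeginPlay it shows the item's name from its Data struct in the info widget.
; Its overridden Interact event wraps Data and Amount in an inventory slot structure and passes it to the interacting actor's InventoryComponent.
; The item destroys itself only if AddToInventory succeeds.
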(event `self.ReceiveBeginPlay`
  ;[1 1 1] Event Beginplay; Set Info Widget Text to display Item Name
  (`self.SetInfoWidgetText` (`.Name_2_FA5597F34D3B5526DD7F79A1F159E53C` (break `/Game/AdventurePack/Blueprints/Utility/ItemStructure` (`self.Data`)))))

(event `/Game/AdventurePack/Blueprints/Interfaces/IInteractable.Interact`
  (params (InteractingActor :type "Actor Object Reference"))
  ;[1 1 1] Overriden Event Interact; Adds Item to Inventory, if success- destroys this actor
  (bind _success_ (`/Game/AdventurePack/Blueprints/Components/InventoryComponent.AddToInventory` (`self.GetComponentByClass` InteractingActor "/Game/AdventurePack/Blueprints/Components/InventoryComponent.InventoryComponent_C") (make `/Game/AdventurePack/Blueprints/Utility/InventorySlotStructure` (`self.Data`) (`self.Amount`))))
  (if _success_
    (`self.K2_DestroyActor`)))

(fn `UserConstructionScript`)