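; Interactable puzzle tile that flips between active and inactive states, shown by swapping the material on its static mesh.
; BeginPlay applies the starting material, and each Interact toggles the state, updates the material and calls OnTileToggled with the new value.
; It then invokes its target actors (adjacent tiles) only when the interacting actor lacks the Interactable interface, so toggles from other interactables do not propagate further.
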(event `self.ReceiveBeginPlay`
  ;[1 1 1] Event Beginplay; Set Color of the tile  based on Active? bool
  (`parent.ReceiveBeginPlay`)
  (`self.SetTileMaterial`))

(event `self.Interact`
  (params (InteractingActor :type "Actor Object Reference"))
  ;[1 1 1] Event Interact; Toggle Active? bool, if interacting actor does not implement Interactable Interface, activate adjacent tiles
  (`self.ToggleTile`)
  (`self.OnTileToggled` (`self.Active?`))
  ;;[1 1 1] Activate adjacent tiles only if interacting actor doesnt have Interactable interface;
  (if (not (`KismetSystemLibrary.DoesImplementInterface` InteractingActor "/Game/AdventurePack/Blueprints/Interfaces/IInteractable.IInteractable_C"))
    (`self.InvokeTargetActors` self)))

(fn `SetTileMaterial`
  (`PrimitiveComponent.SetMaterial` (`self.StaticMesh`) 0 (select `bool` (`self.Active?`) :`false` (`self.InactiveMaterial`) :`true` (`self.ActiveMaterial`))))

(fn `ToggleTile`
  (set `self.Active?` (not (`self.Active?`)))
  (`self.SetTileMaterial`))

(fn `UserConstructionScript`
  (`parent.UserConstructionScript`))