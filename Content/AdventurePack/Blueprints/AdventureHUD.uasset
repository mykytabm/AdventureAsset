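; AdventureHUD Blueprint that owns the on-screen interaction pop-up and hint widgets for the adventure pack.
; On BeginPlay it creates both widgets, adds them to the viewport and hides them.
; Helper functions show, hide or toggle each widget by switching between Visible and Collapsed, and set the interaction type or hint text, so widgets are reused rather than recreated.
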(event `self.ReceiveBeginPlay`
  ;[1 1 1] Event Construct; Create InteractionPopUp Widget, add it to viewport and hide it; Create Hint Widget, add to viewport and hide it
  (`self.CreateInteractionPopupWB`)
  (`self.CreateHintWB`))

(fn `CreateHintWB`
  (bind _returnvalue (`|CreateWidget` "/Game/AdventurePack/Widgets/Interaction/WBHint.WBHint_C"))
  (bind _output_get (set `self.WBHint` _returnvalue))
  (`UserWidget.AddToViewport` _output_get 0)
  (`self.SetHintVisibility` false))

(fn `CreateInteractionPopupWB`
  (bind _returnvalue (`|CreateWidget` "/Game/AdventurePack/Widgets/Interaction/WBInteractionPopUp.WBInteractionPopUp_C"))
  (bind _output_get (set `self.WBInteractionPopUp` _returnvalue))
  (`UserWidget.AddToViewport` _output_get 0)
  (`self.SetInteractionPopUpVisibility` false))

(fn `HideInteractionPopUp`
  (`Widget.SetVisibility` (`self.WBInteractionPopUp`) "Collapsed"))

(fn `SetHintText`
  (params (InText :type Text))
  (`TextBlock.SetText` (`/Game/AdventurePack/Widgets/Interaction/WBHint.HintText` (`self.WBHint`)) InText))

(fn `SetHintVisibility`
  (params (NewVisibility :type Boolean))
  (`Widget.SetVisibility` (`self.WBHint`) (select `bool` NewVisibility :`false` "Collapsed" :`true` "Visible" :!type "ESlateVisibility Enum")))

(fn `SetInteractionPopUpVisibility`
  (params (`newVisible?` :type Boolean))
  (`Widget.SetVisibility` (`self.WBInteractionPopUp`) (select `bool` `newVisible?` :`false` "Collapsed" :`true` "Visible" :!type "ESlateVisibility Enum")))

(fn `ShowInteractionPopUp`
  (params (InteractionTypeText :type Text))
  (bind _wbinteractionpopup (`self.WBInteractionPopUp`))
  (`TextBlock.SetText` (`/Game/AdventurePack/Widgets/Interaction/WBInteractionPopUp.InteractionType` _wbinteractionpopup) InteractionTypeText)
  (`Widget.SetVisibility` _wbinteractionpopup "Visible"))

(fn `UserConstructionScript`)