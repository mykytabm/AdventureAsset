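; BaseInteractable is a base Blueprint for interactable objects, with an InfoWidget component that shows the object's name.
; On BeginPlay it casts the widget to WBInteractableInfo and sets its Info text from Name.
; A helper function toggles the widget's visibility without propagating to children.
; The Interact event receives the interacting actor and is empty in this class.
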(event `self.ReceiveBeginPlay`
  ;[1 1 1] Beginplay; Set InfoWidget Text
  (`self.SetInfoWidgetText`))

(event `Interact`
  (params (InteractingActor :type "Actor Object Reference")))

(fn `SetInfoWidgetText`
  (bind _aswbinteractable_info (cast `/Game/AdventurePack/Widgets/WBInteractableInfo` (`WidgetComponent.GetUserWidgetObject` (`self.InfoWidget`))))
  (`TextBlock.SetText` (`/Game/AdventurePack/Widgets/WBInteractableInfo.Info` _aswbinteractable_info) (`self.Name`)))

(fn `SetInfoWidgetVIsibility`
  (params (bNewVisibility :type Boolean))
  (`SceneComponent.SetVisibility` (`self.InfoWidget`) bNewVisibility false))

(fn `UserConstructionScript`)