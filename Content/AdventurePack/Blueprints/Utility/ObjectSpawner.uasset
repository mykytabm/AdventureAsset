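; ObjectSpawner is a utility Blueprint that lines a spline with static meshes spaced at a set Separation.
; The Construction Script derives the count from spline length divided by Separation, then adds a mesh component at each distance along the spline.
; The first uses FirstMesh, interior ones pick randomly from MiddleMeshes, and the last uses LastMesh yawed 180 degrees, or a random middle mesh if LastMesh is invalid.
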(fn `CalculateNumberOfMeshesToSpawn`
  (returns (Output_Get :type Integer))
  (return (`.ReturnValue` (`KismetMathLibrary.FMod` (`SplineComponent.GetSplineLength` (`self.Spline`)) (`self.Separation`)))))

(fn `UserConstructionScript`
  (locals (`Num of Meshes` :type Integer :default 0) (`Static Mesh Comp` :type "StaticMeshComponent Object Reference"))
  (bind _lastmesh (`self.LastMesh`))
  (bind _middlemeshes (`self.MiddleMeshes`))
  (bind _output_get (`self.CalculateNumberOfMeshesToSpawn`))
  (bind _output_get_2 (set `local.Num of Meshes` _output_get))
  (for _index (range (+ _output_get_2 1))
    (bind _returnvalue (`AddComponent|NODE_AddStaticMeshComponent-2` :`RelativeTransform` (`self.CalculateTransformAlongSplineAtDistance` (`self.Spline`) (* _index (`self.Separation`)))))
    (set `local.Static Mesh Comp` _returnvalue)
    (if (== _index 0)
      ;[1 1 1] Create First Static Mesh
      (`StaticMeshComponent.SetStaticMesh` (`local.Static Mesh Comp`) (`self.FirstMesh`))
      (elif (== _index (`local.Num of Meshes`))
        ;[1 1 1] Create Last Static mesh if its valid
        (`/Engine/EditorBlueprintResources/StandardMacros.IsValid` _lastmesh
          (:`Is Valid`
            (`StaticMeshComponent.SetStaticMesh` (`local.Static Mesh Comp`) _lastmesh)
            (`SceneComponent.K2_SetRelativeRotation` (`local.Static Mesh Comp`) (`KismetMathLibrary.MakeRotator` (.roll (`SceneComponent.RelativeRotation` (`local.Static Mesh Comp`))) (.pitch (`SceneComponent.RelativeRotation` (`local.Static Mesh Comp`))) (+ (.yaw (`SceneComponent.RelativeRotation` (`local.Static Mesh Comp`))) 180.0)) false false))
          (:`Is Not Valid`
            (`StaticMeshComponent.SetStaticMesh` (`local.Static Mesh Comp`) (`|GetArrayItem` _middlemeshes (`KismetMathLibrary.RandomIntegerInRange` 0 (- (`KismetArrayLibrary.Array_Length` _middlemeshes) 1))) :!label _label)))
        (else
          (goto _label))))))