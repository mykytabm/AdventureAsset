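; Actor component that lets its owner find, highlight and interact with nearby actors implementing the Interactable interface.
; Owner overlap events maintain a list of player-usable interactables in range.
; Each tick it skips those blocked by a world line trace and favors the one the owner faces most via dot product.
; The selection shows its info widget and a HUD pop-up naming its interaction type, and Interact forwards the owner to it.
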(event `self.ReceiveBeginPlay`
  (bind _returnvalue (`self.GetOwner`))
  ;[1 1 1] Beginplay; Bind owner begin overlap and end overlap
  (add `Actor.OnActorBeginOverlap` _returnvalue (delegate `OnOwnerBeginOverlap`))
  (add `Actor.OnActorEndOverlap` _returnvalue (delegate `OnOwnerEndOverlap`)))

(event `OnOwnerBeginOverlap`
  (params (OverlappedActor :type "Actor Object Reference") (OtherActor :type "Actor Object Reference"))
  ;[1 1 1] On Owner Begin Overlap Event; Add other actor to interactable objects array if actor implements Interactable Interface
  (if (`KismetSystemLibrary.DoesImplementInterface` OtherActor "/Game/AdventurePack/Blueprints/Interfaces/IInteractable.IInteractable_C")
    (bind _usablebyplayer_ (message `/Game/AdventurePack/Blueprints/Interfaces/IInteractable.IsUsableByPlayer?` OtherActor))
    (if _usablebyplayer_
      (`KismetArrayLibrary.Array_Add` (`self.InteractablesAroundOwner`) OtherActor))))

(event `OnOwnerEndOverlap`
  (params (OverlappedActor :type "Actor Object Reference") (OtherActor :type "Actor Object Reference"))
  ;[1 1 1] On Owner End Overlap Event; Remove other actor from interactable objects array if actor implements Interactable Interface
  (if (`KismetSystemLibrary.DoesImplementInterface` OtherActor "/Game/AdventurePack/Blueprints/Interfaces/IInteractable.IInteractable_C")
    (`KismetArrayLibrary.Array_RemoveItem` (`self.InteractablesAroundOwner`) OtherActor)
    (message `/Game/AdventurePack/Blueprints/Interfaces/IInteractable.SetInteractableInfoVisibility` OtherActor false)
    (if (== (`self.SelectedInteractable`) OtherActor)
      (set `self.SelectedInteractable` null))))

(event `self.ReceiveTick`
  (params (DeltaSeconds :type "Float (single-precision)"))
  ;[1 1 1] Event Tick
  (bind _selectedinteractable (`self.SelectInteractableAndHandleWidgetDisabling`))
  (bind _output_get (set `self.SelectedInteractable` _selectedinteractable))
  (`/Engine/EditorBlueprintResources/StandardMacros.IsValid` _output_get
    (:`Is Valid`
      (message `/Game/AdventurePack/Blueprints/Interfaces/IInteractable.SetInteractableInfoVisibility` (`self.SelectedInteractable`) true)
      (bind _interactiontype (message `/Game/AdventurePack/Blueprints/Interfaces/IInteractable.GetInteractionType` (`self.SelectedInteractable`)))
      (`self.SetInteractionPopUpVisibility` true (`KismetTextLibrary.Conv_StringToText` (`|GetEnumeratorNameAsString` _interactiontype))))
    (:`Is Not Valid`
      (`self.SetInteractionPopUpVisibility` false))))

(fn `Interact`
  (`/Engine/EditorBlueprintResources/StandardMacros.IsValid` (`self.SelectedInteractable`)
    (:`Is Valid`
      (message `/Game/AdventurePack/Blueprints/Interfaces/IInteractable.Interact` (`self.SelectedInteractable`) (`self.GetOwner`)))))

(fn `SelectInteractableAndHandleWidgetDisabling`
  (returns (SelectedInteractable :type "Actor Object Reference"))
  (locals (LSelectedInteractable :type "Actor Object Reference") (LArrayElement :type "Actor Object Reference"))
  (set `local.LSelectedInteractable` null)
  (for _array_element (`self.InteractablesAroundOwner`)
    (bind _output_get (set `local.LArrayElement` _array_element))
    (bind _hitobstacle_ (`self.LineTraceFromOwnerToInteractable` _output_get (`|MakeArray` "ObjectTypeQuery1" "ObjectTypeQuery2" :!type "EObjectTypeQuery Enum")))
    (if _hitobstacle_
      ;[1 1 1] Hide Interactable Widget
      (message `/Game/AdventurePack/Blueprints/Interfaces/IInteractable.SetInteractableInfoVisibility` (`local.LArrayElement`) false)
      (else
        (`/Engine/EditorBlueprintResources/StandardMacros.IsValid` (`local.LSelectedInteractable`)
          (:`Is Valid`
            (if (> (`Actor.GetDotProductTo` (`self.GetOwner`) (`local.LArrayElement`)) (`Actor.GetDotProductTo` (`self.GetOwner`) (`local.LSelectedInteractable`)))
              ;[1 1 1] Hide Interactable Widget
              (message `/Game/AdventurePack/Blueprints/Interfaces/IInteractable.SetInteractableInfoVisibility` (`self.SelectedInteractable`) false)
              ;[1 1 1] Set LSelected Interactable
              (set `local.LSelectedInteractable` (`local.LArrayElement`))
              (else
                ;[1 1 1] Hide Interactable Widget
                (message `/Game/AdventurePack/Blueprints/Interfaces/IInteractable.SetInteractableInfoVisibility` (`self.SelectedInteractable`) false))))
          (:`Is Not Valid`
            (set `local.LSelectedInteractable` (`local.LArrayElement`)))))))
  (return (`local.LSelectedInteractable`)))

(fn `SetInteractionPopUpVisibility`
  (params (`newVisible?` :type Boolean) (InText :type Text))
  (bind _asadventure_hud (cast `/Game/AdventurePack/Blueprints/AdventureHUD` (`PlayerController.GetHUD` (`GameplayStatics.GetPlayerController` 0))))
  (`/Game/AdventurePack/Blueprints/AdventureHUD.SetInteractionPopUpVisibility` _asadventure_hud `newVisible?`)
  (`TextBlock.SetText` (`/Game/AdventurePack/Widgets/WBInteractionPopup.InteractionType` (`/Game/AdventurePack/Blueprints/AdventureHUD.WBInteractionPopUp` _asadventure_hud)) InText))