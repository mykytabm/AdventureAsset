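; Component that displays a timed text hint on the player's HUD in the adventure pack.
; DisplayHint, which has a ShowOnce branch with a DoOnce node, sets HintText and visibility through AdventureHUD on player controller 0.
; A non-looping timer then hides the hint and clears its text after ShowHintForSeconds.
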(event `DisplayHint`
  ;[1 1 1] Display Hint Event;  ShowHint And
  (if (`self.ShowOnce?`)
    (`/Engine/EditorBlueprintResources/StandardMacros.DoOnce` false
      (:`Completed`
        _)))
  (bind _success_ (`self.SetHintWidgetText` (`self.HintText`)))
  (if _success_
    (`self.ShowHintWidget`)
    (`KismetSystemLibrary.K2_SetTimerDelegate` (delegate `OnHintTimerTimeout`) (`self.ShowHintForSeconds`))))

(event `OnHintTimerTimeout`
  ;[1 1 1] Display Hint Event;  ShowHint And
  (`self.HideHintWidget`)
  (`self.SetHintWidgetText` ""))

(fn `HideHintWidget`
  (bind _asadventure_hud (cast `/Game/AdventurePack/Blueprints/AdventureHUD` (`PlayerController.GetHUD` (`GameplayStatics.GetPlayerController` 0))))
  (`/Game/AdventurePack/Blueprints/AdventureHUD.SetHintText` _asadventure_hud "")
  (`/Game/AdventurePack/Blueprints/AdventureHUD.SetHintVisibility` _asadventure_hud false))

(fn `SetHintWidgetText`
  (params (pHintText :type Text))
  (returns (`Success?` :type Boolean))
  (bind _asadventure_hud (cast `/Game/AdventurePack/Blueprints/AdventureHUD` (`PlayerController.GetHUD` (`GameplayStatics.GetPlayerController` 0)))
    (:`then`
      (`/Game/AdventurePack/Blueprints/AdventureHUD.SetHintText` _asadventure_hud pHintText)
      (return true))
    (:`CastFailed`
      (return false))))

(fn `ShowHintWidget`
  (returns (`Success?` :type Boolean))
  (bind _asadventure_hud (cast `/Game/AdventurePack/Blueprints/AdventureHUD` (`PlayerController.GetHUD` (`GameplayStatics.GetPlayerController` 0)))
    (:`then`
      (`/Game/AdventurePack/Blueprints/AdventureHUD.SetHintVisibility` _asadventure_hud true)
      (return true))
    (:`CastFailed`
      (`KismetSystemLibrary.PrintString` "Cast to Adventure HUD failed" false)
      (return false))))